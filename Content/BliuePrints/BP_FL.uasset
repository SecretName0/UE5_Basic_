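; BP_FL is a Blueprint function library of small practice functions that act like C++ static functions.
; BP_체력 관리 returns the sum of base and additional health.
; BP_Swap exchanges two variables through a temporary and by-reference sets, so the caller's values can change.
; 함수A, 함수B and 함수C form a nested call chain, each printing start and end text to show call-stack order.
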(fn BP체력관리
  (params (기초%20체력 :type Integer) (추가%20체력 :type Integer))
  (return (+ 기초%20체력 추가%20체력)))

(fn BPSwap
  (params (변수1 :type Integer%20%28by%20ref%29) (변수2 :type Integer%20%28by%20ref%29))
  (LocalVariables|SetTemp 변수1)
  (|SetBy-RefVar 변수1 변수2) ; 타겟을 밸류 값으로 교체한다.\n즉, 이것은 현재 변수1이 2로 덮어 씌워짐
  (|SetBy-RefVar 변수2 (LocalVariables|GetTemp)) ; 타겟을 밸류 값으로 교체한다.\n이것은 변수2가 Temp로 덮어씌워짐
)

(fn 함수A
  (Development|PrintText 0 "A시작")
  (CallFunction|함수B)
  (Development|PrintText 0 "A끝"))

(fn 함수B
  (Development|PrintText 0 "B시작")
  (CallFunction|함수C)
  (Development|PrintText 0 "B끝"))

(fn 함수C
  (Development|PrintText 0 "C시작")
  (Development|PrintText 0 "C끝"))